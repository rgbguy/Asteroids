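; Bullet_BP is a projectile for the Asteroids game that destroys asteroid-game actors it touches.
; Each Tick moves its Sphere component along the forward vector by SpeedMultiplier, without sweep or delta-time scaling.
; An overlap with an AsteroidsBase_BP actor calls that actor's Death and destroys the bullet.
; It also destroys itself a fixed delay after spawning.
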(event `self.ReceiveBeginPlay`
  (`KismetSystemLibrary.Delay` 8.0)
  (`self.K2_DestroyActor`))

(event `self.Sphere.OnComponentBeginOverlap`
  (params (OverlappedComponent :type "PrimitiveComponent Object Reference") (OtherActor :type "Actor Object Reference") (OtherComp :type "PrimitiveComponent Object Reference") (OtherBodyIndex :type Integer) (bFromSweep :type Boolean) (SweepResult :type "HitResult Structure (by ref)"))
  (bind _asasteroids_base_bp (cast `/Game/Asteroids/AsteroidsBase_BP` OtherActor))
  (`/Game/Asteroids/AsteroidsBase_BP.Death` _asasteroids_base_bp)
  (`self.K2_DestroyActor`))

(event `self.ReceiveTick`
  (params (DeltaSeconds :type "Float (single-precision)"))
  (bind _sphere (`self.Sphere`))
  (`SceneComponent.K2_AddWorldOffset` _sphere (* (`self.SpeedMultiplier`) (`SceneComponent.GetForwardVector` _sphere)) false false))

(fn `UserConstructionScript`)