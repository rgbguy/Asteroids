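; Base asteroid actor that drifts across the play area and splits into smaller asteroids when destroyed.
; BeginPlay picks a random XY direction, and Tick offsets the AsteroidL0 component along it by SpeedMultiplier per frame, without sweep or delta-time scaling.
; Death spawns two Asteroid_L1_BP actors at that component's transform, plays an explosion sound and destroys the actor.
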(event `self.ReceiveBeginPlay`
  (set `self.RandomDirectionToThrow` (`KismetMathLibrary.MakeVector` (`KismetMathLibrary.RandomFloatInRange` -1.0 1.0) (`KismetMathLibrary.RandomFloatInRange` -1.0 1.0))))

(event `self.ReceiveTick`
  (params (DeltaSeconds :type "Float (single-precision)"))
  (`SceneComponent.K2_AddWorldOffset` (`self.Asteroid_L0`) (* (`self.RandomDirectionToThrow`) (`self.SpeedMultiplier`)) false false))

(fn `Death`
  (`|SpawnActorFromClass` "/Game/Asteroids/Asteroid_L1_BP.Asteroid_L1_BP_C" (`SceneComponent.K2_GetComponentToWorld` (`self.Asteroid_L0`)) "AdjustIfPossibleButAlwaysSpawn" "MultiplyWithRoot" null null)
  (`|SpawnActorFromClass` "/Game/Asteroids/Asteroid_L1_BP.Asteroid_L1_BP_C" (`SceneComponent.K2_GetComponentToWorld` (`self.Asteroid_L0`)) "AdjustIfPossibleButAlwaysSpawn" "MultiplyWithRoot" null null)
  (`GameplayStatics.PlaySound2D` "/Game/Asteroids/Sounds/Explosion24.Explosion24" 1.0 1.0 0.0 null null)
  (`self.K2_DestroyActor`))

(fn `UserConstructionScript`)