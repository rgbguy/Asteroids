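; Large-tier asteroid Blueprint that breaks into smaller asteroids when it dies.
; On BeginPlay it runs the parent logic, then sets its speed multiplier.
; Death spawns two Asteroids_L2_BP actors at the AsteroidL0 component's transform, nudging them if needed but always spawning, then destroys itself.
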(event `self.ReceiveBeginPlay`
  (`parent.ReceiveBeginPlay`)
  (set `self.SpeedMultiplier` 10.0))

(fn `Death`
  (`|SpawnActorFromClass` "/Game/Asteroids/Asteroids_L2_BP.Asteroids_L2_BP_C" (`SceneComponent.K2_GetComponentToWorld` (`self.Asteroid_L0`)) "AdjustIfPossibleButAlwaysSpawn" "MultiplyWithRoot" null null)
  (`|SpawnActorFromClass` "/Game/Asteroids/Asteroids_L2_BP.Asteroids_L2_BP_C" (`SceneComponent.K2_GetComponentToWorld` (`self.Asteroid_L0`)) "AdjustIfPossibleButAlwaysSpawn" "MultiplyWithRoot" null null)
  (`self.K2_DestroyActor`))

(fn `UserConstructionScript`
  (`parent.UserConstructionScript`))